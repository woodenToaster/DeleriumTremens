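; DTCamera is a camera Blueprint that watches for viewport size changes so the game screen can be resized to match.
; BeginPlay caches the GlobalDTGameInstance, and CheckViewport compares the viewport size to its stored value, publishing changes to that instance.
; DoOnce gates guard the Resize call on the stored game screen.
; UpdateCamera is an empty stub, and nothing here calls CheckViewport.
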(event EventBeginPlay
  (bind _asglobal_dtgame_instance (Utilities|Casting|CastToGlobalDTGameInstance (Game|GetGameInstance)))
  (Variables|Default|SetStoredGameInstance _asglobal_dtgame_instance))

(event Collision|EventActorBeginOverlap
  (params (OtherActor :type Actor%20Object%20Reference)))

(event EventTick
  (params (DeltaSeconds :type Float%20%28single-precision%29)))

(fn ConstructionScript)

(fn CheckViewport
  (bind _returnvalue (Viewport|GetViewportSize))
  (bind _returnvalue_2 (Viewport|GetViewportSize))
  (if (Utilities|IsValid (Variables|Default|GetStoredGameInstance))
    _
    (else
      (bind _asglobal_dtgame_instance (Utilities|Casting|CastToGlobalDTGameInstance (Game|GetGameInstance)))
      (Variables|Default|SetStoredGameInstance _asglobal_dtgame_instance)))
  (Utilities|FlowControl|Sequence
    (:then_0
      (if (or (!= (.x _returnvalue_2) (.x (Variables|Default|GetStoredSize))) (!= (.y _returnvalue_2) (.y (Variables|Default|GetStoredSize))))
        (bind _output_get (Variables|Default|SetStoredSize (Math|Vector2D|MakeVector2D (.x _returnvalue_2) (.y _returnvalue_2))))
        (Variables|/Game/Blueprints/GlobalDTGameInstance.GlobalDTGameInstance_C|SetStoredCameraRez (Variables|Default|GetStoredGameInstance) _output_get)
        (Utilities|FlowControl|Sequence
          (:then_0
            (Utilities|FlowControl|DoOnce false :!label _label
              (:Completed
                (CallFunction|UpdateCamera)
                (Utilities|Casting|CastToGameLevelGameMode (Game|GetGameMode))
                (Default|Resize (Variables|/Game/Blueprints/GlobalDTGameInstance.GlobalDTGameInstance_C|GetStoredGameScreen (Variables|Default|GetStoredGameInstance)) :!label _label_2)
                (Development|PrintString "Resize Called")
                (return))))
          (:then_1
            (goto _label_3 Reset)))))
    (:then_1
      (if (and (!= (.x _returnvalue) 0.0) (!= (.y _returnvalue) 0.0))
        (goto _label)))
    (:then_2
      (if (Utilities|IsValid (Variables|/Game/Blueprints/GlobalDTGameInstance.GlobalDTGameInstance_C|GetStoredGameScreen (Variables|Default|GetStoredGameInstance)))
        (Utilities|FlowControl|DoOnce false :!label _label_3
          (:Completed
            (goto _label_2)))))))

(fn UpdateCamera
  (return))